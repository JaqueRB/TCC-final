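; Anubis statue actor that shows a prompt widget component while the player is nearby and can open the Wb_Anubis screen.
; Sphere overlaps with Bp_player toggle the widget's visibility and the IsinSphere flag.
; The AbrirWidgter event, not called within this graph, adds Wb_Anubis to the viewport and shows the mouse cursor while setting game-only input.
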(event OnComponentBeginOverlap(Sphere)
  (params (OverlappedComponent :type Primitive%20Component%20Object%20Reference) (OtherActor :type Actor%20Object%20Reference) (OtherComp :type Primitive%20Component%20Object%20Reference) (OtherBodyIndex :type Integer) (bFromSweep :type Boolean) (SweepResult :type Hit%20Result%20Structure%20%28by%20ref%29))
  (Utilities|Casting|CastToBp_player OtherActor)
  (Rendering|SetVisibility (Variables|Default|GetWidget) true false)
  (Variables|Default|SetisinSphere? true))

(event OnComponentEndOverlap(Sphere)
  (params (OverlappedComponent :type Primitive%20Component%20Object%20Reference) (OtherActor :type Actor%20Object%20Reference) (OtherComp :type Primitive%20Component%20Object%20Reference) (OtherBodyIndex :type Integer))
  (Utilities|Casting|CastToBp_player OtherActor)
  (Rendering|SetVisibility (Variables|Default|GetWidget) false false)
  (Variables|Default|SetisinSphere? false))

(event Custom|AbrirWidgter
  (bind _returnvalue (UserInterface|CreateWidget "/Game/Dialogo_Interativo/Wb_Anubis.Wb_Anubis_C"))
  (UserInterface|Viewport|AddtoViewport _returnvalue 0)
  (Input|SetInputModeGameOnly)
  (Variables|/Script/Engine.PlayerController|SetbShowMouseCursor (Game|GetPlayerController 0) true))

(fn ConstructionScript)