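; Player character for an Egyptian-themed puzzle game, handling movement, jumping, pause menu, timed intro dialogue and a countdown to game over.
; Camera line traces drive E interactions with per-type actors, F/Q tumbler lock spins and right-mouse Physics Handle grabbing of light objects.
; R opens the first puzzle's widget, which receives parts through Agregarparte.
; Tick moves held objects and uses a Delay to step the timer each second.
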(event Custom|Agregar%20parte
  (params (parte :type Estructura%20Parte%20Structure))
  ;[0.6824 0.302 1] Puzzle 1 (linkar 2 funções para que o puzzle possa ser aberto corretamente)
  (Default|Agregarparte (Variables|Default|Getwidget_puzzle) parte))

(event EventBeginPlay
  (Utilities|FlowControl|Sequence
    (:then_0
      ;[1 0 0] Menu de pause
      (bind _returnvalue (UserInterface|CreateWidget "/Game/Menu_pause/menu_pause.menu_pause_C"))
      (Variables|Default|SetRef%20pause _returnvalue))
    (:then_1
      ;[0.6824 0.302 1] Puzzle 1(aparecer tela para o player conseguir realizar o puzzle
      (bind _returnvalue_2 (UserInterface|CreateWidget "/Game/StarterContent/Puzzle1/Wb_puzzle.Wb_puzzle_C" (Game|GetPlayerController 0)))
      (Variables|Default|Setwidget_puzzle _returnvalue_2))
    (:then_2
      ;[0.4557 1 0.2946] Dialogo
      (bind _returnvalue_3 (UserInterface|CreateWidget "/Game/dialogo/dialogo_inicio.dialogo_inicio_C"))
      (UserInterface|Viewport|AddtoViewport _returnvalue_3 0)
      (Utilities|FlowControl|Delay 35.0)
      (Widget|RemovefromParent _returnvalue_3))))

(event EventTick
  (params (DeltaSeconds :type Float%20%28single-precision%29))
  (bind _camera (Variables|Default|GetCamera))
  (Utilities|FlowControl|Sequence
    (:then_0
      ;[1 0.5272 0.04774] Tempo
      (Utilities|FlowControl|Delay 1.0)
      (if (== (Variables|Default|Getsegundos) 0)
        (if (== (Variables|Default|Getminutos) 0)
          (bind _returnvalue (UserInterface|CreateWidget "/Game/Timer/Game_Over.Game_Over_C"))
          (UserInterface|Viewport|AddtoViewport _returnvalue 0)
          (Variables|/Script/Engine.PlayerController|SetbShowMouseCursor (Game|GetPlayerController 0) true)
          (Game|SetGamePaused true)
          (else
            (Variables|Default|Setsegundos 59)
            (Variables|Default|Setminutos (- (Variables|Default|Getminutos) 1))))
        (else
          (Variables|Default|Setsegundos (- (Variables|Default|Getsegundos) 1)))))
    (:then_1
      ;[0 0.6724 1] Objeto na mão (loop) [Puzzle3]
      (if (Variables|Default|GetSegurandoObjeto)
        (Physics|Components|PhysicsHandle|SetTargetLocation (Variables|Default|GetPhysicsHandle) (+ (Transformation|GetWorldLocation _camera) (* (Math|Vector|GetForwardVector _camera) 2e+02)))))))

(event Input|AxisEvents|InputAxisfrente_tras
  (params (AxisValue :type Float%20%28single-precision%29))
  ;[0.01569 0.1686 1] movimentação teclado
  (Pawn|Input|AddMovementInput (Math|Vector|GetForwardVector (Math|Rotator|MakeRotator 0.0 0.0 (.Yaw (Math|Rotator|BreakRotator (Pawn|GetControlRotation :!class /Script/Engine.Pawn))))) AxisValue false))

(event Input|AxisEvents|InputAxisdireita_esquerda
  (params (AxisValue :type Float%20%28single-precision%29))
  ;[0.01569 0.1686 1] movimentação teclado
  (Pawn|Input|AddMovementInput (Math|Vector|GetRightVector (Math|Rotator|MakeRotator 0.0 0.0 (.Yaw (Math|Rotator|BreakRotator (Pawn|GetControlRotation :!class /Script/Engine.Pawn))))) AxisValue false))

(event Input|AxisEvents|InputAxisMouse_direita
  (params (AxisValue :type Float%20%28single-precision%29))
  ;[0.01569 0.1686 1] controle mouse
  (bind _asbp_player (Utilities|Casting|CastToBp_player (Game|GetPlayerCharacter 0)))
  (Pawn|Input|AddControllerYawInput _asbp_player AxisValue))

(event Input|AxisEvents|InputAxismouse_cima_baixo
  (params (AxisValue :type Float%20%28single-precision%29))
  ;[0.01569 0.1686 1] controle mouse
  (bind _asbp_player (Utilities|Casting|CastToBp_player (Game|GetPlayerCharacter 0)))
  (Pawn|Input|AddControllerPitchInput _asbp_player AxisValue))

(event Input|KeyboardEvents|R
  (params (Key :type Key%20Structure :default "None"))
  (bind _returnvalue (Game|GetPlayerController 0))
  ;[0.6824 0.302 1] comando para aparecer a tela de fazer o puzzle 1
  (:Pressed
    (UserInterface|Viewport|AddtoPlayerScreen (Variables|Default|Getwidget_puzzle))
    (Input|SetInputModeUIOnly _returnvalue 0 "DoNotLock")
    (Variables|/Script/Engine.PlayerController|SetbShowMouseCursor _returnvalue true)))

(event Input|KeyboardEvents|SpaceBar
  (params (Key :type Key%20Structure :default "None"))
  ;[0.01569 0.1686 1] Pular
  (:Pressed
    (Character|Jump)))

(event Input|KeyboardEvents|E
  (params (Key :type Key%20Structure :default "None"))
  (bind _camera (Variables|Default|GetCamera))
  (bind _returnvalue (Transformation|GetWorldLocation _camera))
  ;[1 1 1] Interativo Esfinge
  (:Pressed
    (if true
      (bind (_outhit _returnvalue_2) (Collision|LineTraceByChannel _returnvalue (+ _returnvalue (* (Math|Vector|GetForwardVector _camera) 2e+02)) "TraceTypeQuery1" false 0 "None"))
      (if _returnvalue_2
        (bind _asinteract_actor_esfinge (Utilities|Casting|CastToInteractActor_esfinge (.HitActor (Collision|BreakHitResult _outhit))))
        (Default|AbrirWidgter _asinteract_actor_esfinge)))))

(event Input|MouseEvents|RightMouseButton
  (params (Key :type Key%20Structure :default "None"))
  (bind _camera (Variables|Default|GetCamera))
  (bind _returnvalue (Transformation|GetWorldLocation _camera))
  ;[0 0.6724 1] Sistema de pegar Objeto [Puzzle 3]
  (:Pressed
    (bind (_outhit _returnvalue_2) (Collision|LineTraceByChannel _returnvalue (+ _returnvalue (* (Math|Vector|GetForwardVector _camera) 2e+02)) "TraceTypeQuery1" false 0 "None"))
    (if _returnvalue_2
      (if (< (Physics|GetMass (.HitComponent (Collision|BreakHitResult _outhit))) 1.5e+02)
        (Physics|Components|PhysicsHandle|GrabComponentatLocationwithRotation (Variables|Default|GetPhysicsHandle) (.HitComponent (Collision|BreakHitResult _outhit)) "None" (Transformation|GetWorldLocation (.HitComponent (Collision|BreakHitResult _outhit))) "0, 0, 0")
        (Variables|Default|SetSegurandoObjeto true))))
  (:Released
    (if (Variables|Default|GetSegurandoObjeto)
      (Physics|Components|PhysicsHandle|ReleaseComponent (Variables|Default|GetPhysicsHandle))
      (Variables|Default|SetSegurandoObjeto false))))

(event Input|KeyboardEvents|E
  (params (Key :type Key%20Structure :default "None"))
  (bind _camera (Variables|Default|GetCamera))
  (bind _returnvalue (Transformation|GetWorldLocation _camera))
  ;[1 1 1] Interativo Puzzle 1
  (:Pressed
    (if true
      (bind (_outhit _returnvalue_2) (Collision|LineTraceByChannel _returnvalue (+ _returnvalue (* (Math|Vector|GetForwardVector _camera) 2e+02)) "TraceTypeQuery1" false 0 "None"))
      (if _returnvalue_2
        (bind _asinteract_actor (Utilities|Casting|CastTointeract_actor (.HitActor (Collision|BreakHitResult _outhit))))
        (Default|AbrirWidgter _asinteract_actor)))))

(event Input|KeyboardEvents|F
  (params (Key :type Key%20Structure :default "None"))
  (bind _camera (Variables|Default|GetCamera))
  (bind _returnvalue (Transformation|GetWorldLocation _camera))
  ;[0 1 0.05098] Comando Passar para frente Puzzle2
  (:Pressed
    (if (Variables|Default|GetUsingLock?)
      (if (== (Variables|Default|Getgraus) 360)
        (bind (_outhit _returnvalue_2) (Collision|LineTraceByChannel _returnvalue (+ _returnvalue (* (Math|Vector|GetForwardVector _camera) 2e+02)) "TraceTypeQuery1" false 0 "None"))
        (if _returnvalue_2
          (if (Utilities|IsValid (.HitActor (Collision|BreakHitResult _outhit)))
            (if (Actor|ActorHasTag (.HitActor (Collision|BreakHitResult _outhit)) "Tumbler")
              (bind _asbp_locktumbler (Utilities|Casting|CastToBP_locktumbler (.HitActor (Collision|BreakHitResult _outhit))))
              (Default|SpinTumbler _asbp_locktumbler)))))
      (else
        (Variables|Default|SetUsingLock? false)))))

(event Input|KeyboardEvents|Tab
  (params (Key :type Key%20Structure :default "None"))
  ;[1 0 0] Menu de pause
  (:Pressed
    (Utilities|FlowControl|FlipFlop
      (:A
        (Variables|/Script/Engine.PlayerController|SetbShowMouseCursor (Game|GetPlayerController 0) true)
        (Game|SetGamePaused true)
        (UserInterface|Viewport|AddtoViewport (Variables|Default|GetRef%20pause) 0))
      (:B
        (Variables|/Script/Engine.PlayerController|SetbShowMouseCursor (Game|GetPlayerController 0) false)
        (Game|SetGamePaused false)
        (Widget|RemovefromParent (Variables|Default|GetRef%20pause))))))

(event Input|KeyboardEvents|Q
  (params (Key :type Key%20Structure :default "None"))
  (bind _camera (Variables|Default|GetCamera))
  (bind _returnvalue (Transformation|GetWorldLocation _camera))
  ;[0 1 0.05098] Comando passar para trás puzzle2
  (:Pressed
    (if (Variables|Default|GetUsingLock?)
      (if (== (Variables|Default|Getgraus) 360)
        (bind (_outhit _returnvalue_2) (Collision|LineTraceByChannel _returnvalue (+ _returnvalue (* (Math|Vector|GetForwardVector _camera) 2e+02)) "TraceTypeQuery1" false 0 "None"))
        (if _returnvalue_2
          (if (Utilities|IsValid (.HitActor (Collision|BreakHitResult _outhit)))
            (if (Actor|ActorHasTag (.HitActor (Collision|BreakHitResult _outhit)) "Tumbler")
              (bind _asbp_locktumbler (Utilities|Casting|CastToBP_locktumbler (.HitActor (Collision|BreakHitResult _outhit))))
              (Default|Spintumblerbackward _asbp_locktumbler)))))
      (else
        (Variables|Default|SetUsingLock? false)))))

(event Input|KeyboardEvents|E
  (params (Key :type Key%20Structure :default "None"))
  (bind _camera (Variables|Default|GetCamera))
  (bind _returnvalue (Transformation|GetWorldLocation _camera))
  ;[1 1 1] interativo Pirâmides Gizé
  (:Pressed
    (if true
      (bind (_outhit _returnvalue_2) (Collision|LineTraceByChannel _returnvalue (+ _returnvalue (* (Math|Vector|GetForwardVector _camera) 2e+02)) "TraceTypeQuery1" false 0 "None"))
      (if _returnvalue_2
        (bind _asinteract_actor_pyramids (Utilities|Casting|CastToInteractActor_Pyramids (.HitActor (Collision|BreakHitResult _outhit))))
        (Default|AbrirWidgter _asinteract_actor_pyramids)))))

(event Input|KeyboardEvents|E
  (params (Key :type Key%20Structure :default "None"))
  (bind _camera (Variables|Default|GetCamera))
  (bind _returnvalue (Transformation|GetWorldLocation _camera))
  ;[1 1 1] Interativo Estatuas
  (:Pressed
    (if true
      (bind (_outhit _returnvalue_2) (Collision|LineTraceByChannel _returnvalue (+ _returnvalue (* (Math|Vector|GetForwardVector _camera) 2e+02)) "TraceTypeQuery1" false 0 "None"))
      (if _returnvalue_2
        (bind _asinteract_actor_estatuas (Utilities|Casting|CastToInteractActor_Estatuas (.HitActor (Collision|BreakHitResult _outhit))))
        (Default|AbrirWidgter _asinteract_actor_estatuas)))))

(event Input|KeyboardEvents|E
  (params (Key :type Key%20Structure :default "None"))
  (bind _camera (Variables|Default|GetCamera))
  (bind _returnvalue (Transformation|GetWorldLocation _camera))
  ;[1 1 1] Interativo Estátua do Anubis
  (:Pressed
    (if true
      (bind (_outhit _returnvalue_2) (Collision|LineTraceByChannel _returnvalue (+ _returnvalue (* (Math|Vector|GetForwardVector _camera) 2e+02)) "TraceTypeQuery1" false 0 "None"))
      (if _returnvalue_2
        (bind _asinteract_actor_anubis (Utilities|Casting|CastToInteractActor_anubis (.HitActor (Collision|BreakHitResult _outhit))))
        (Default|AbrirWidgter _asinteract_actor_anubis)))))

(fn ConstructionScript)

(fn OnRepOverlappedInteractor)